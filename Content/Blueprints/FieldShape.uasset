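; FieldShape is an actor that represents a multi-tile shape as a map of 2D integer points and shows it with spawned ShapeTile actors.
; BeginPlay picks a shape through a time-seeded random switch with only a four-tile line case, then refreshes the visuals.
; The refresh destroys child components of Tiles, then attaches one tile per point, offset in X/Y.
; Left and right rotation are empty stubs.
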(event EventBeginPlay
  (bind _seconds (Class|GameplayStatics|GetAccurateRealTime))
  (bind _returnvalue (Math|Random|MakeRandomStream _seconds))
  (switch int (Math|Random|RandomIntegerinRangefromStream 0 0 _returnvalue)
    (:0
      (Variables|Default|SetPoints (|Make4XLineShape _returnvalue))
      (CallFunction|UpdateTilesVisual))))

(event Collision|EventActorBeginOverlap
  (params (OtherActor :type Actor%20Object%20Reference)))

(event EventTick
  (params (DeltaSeconds :type Float%20%28single-precision%29)))

(fn ConstructionScript)

(fn RotateShapeLeft)

(fn RotateShapeRight)

(fn UpdateTilesVisual
  (bind _returnvalue (Transformation|GetWorldLocation))
  (bind (_x _y _z) (Math|Vector|BreakVector _returnvalue))
  (Utilities|FlowControl|Sequence
    (:then_0
      (|DeleteOldVisual))
    (:then_1
      (bind _keys (Utilities|Map|Keys (Variables|Default|GetPoints)))
      (for _array_element _keys
        (bind _returnvalue_2 (Game|SpawnActorfromClass "/Game/Blueprints/ShapeTile.ShapeTile_C" (Math|Transform|MakeTransform "0, 0, 0") "Undefined" 0 0))
        (Transformation|AttachActorToActor _returnvalue_2 (Variables|/Script/Engine.ChildActorComponent|GetChildActor (Variables|Default|GetTiles)) "None" "KeepRelative" "KeepRelative" "KeepRelative" true)
        (Transformation|SetActorLocation _returnvalue_2 (Math|Vector|MakeVector (+ _x (Math|Conversions|ToFloat(Integer) (.X (Utilities|Struct|BreakIntVector2D _array_element)))) (+ (Math|Conversions|ToFloat(Integer) (.Y (Utilities|Struct|BreakIntVector2D _array_element))) _y) _z) false false)))))