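; Camera controller actor that drives an orthographic scene capture for the game's Tetris and dungeon modes.
; On BeginPlay it hides its GameOver component and registers itself with MainGameMode.
; Each tick it eases ortho width and position toward the fixed Tetris framing or the player's Y/Z in the dungeon, per MainGameState.
; It scales the whole actor by ortho width relative to Tetris size, so attached components follow the zoom.
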(event EventBeginPlay
  (Rendering|SetVisibility (Variables|Default|GetGameOver) false false)
  (Variables|/Game/Blueprints/MainGameMode.MainGameMode_C|SetCameraController (.AsMain%20Game%20Mode (Utilities|Casting|CastToMainGameMode (Game|GetGameMode))) self))

(event Collision|EventActorBeginOverlap
  (params (OtherActor :type Actor%20Object%20Reference)))

(event EventTick
  (params (DeltaSeconds :type Float%20%28single-precision%29))
  (bind _returnvalue (Game|GetGameState))
  (bind _returnvalue_2 (Game|GetGameMode))
  (bind _tetrisposition (Variables|Default|GetTetrisPosition))
  (bind _scenecapturecomponent2d (Variables|Default|GetSceneCaptureComponent2D))
  (bind _interptime (Variables|Default|GetInterpTime))
  (bind _returnvalue_3 (/ DeltaSeconds _interptime))
  (bind _asmain_game_state (Utilities|Casting|CastToMainGameState _returnvalue))
  (bind _asmain_game_mode (Utilities|Casting|CastToMainGameMode _returnvalue_2))
  (bind _combat_controller (Variables|/Game/Blueprints/MainGameMode.MainGameMode_C|GetCombat%20Controller _asmain_game_mode))
  (bind _istetrismode (Variables|/Game/Blueprints/MainGameState.MainGameState_C|GetIsTetrisMode _asmain_game_state))
  (bind _playerptr (Variables|/Game/Blueprints/Combat/CombatController.CombatController_C|GetPlayerPtr _combat_controller))
  (bind _returnvalue_4 (Transformation|GetActorLocation _playerptr))
  (Utilities|FlowControl|Sequence
    (:then_0
      (bind _output_get (Variables|Default|SetTargetOrthoSize (select _istetrismode (Variables|Default|GetTetrisOrtoSize) (Variables|Default|GetDungeonOrtoSize))))
      (Variables|/Script/Engine.SceneCaptureComponent2D|SetOrthoWidth _scenecapturecomponent2d (Math|Float|Lerp (Variables|/Script/Engine.SceneCaptureComponent2D|GetOrthoWidth _scenecapturecomponent2d) _output_get _returnvalue_3))
      (if _istetrismode
        (bind _output_get_2 (Variables|Default|SetTargetPosition _tetrisposition))
        (else
          (Variables|Default|SetTargetPosition (select _istetrismode _tetrisposition (Math|Vector|MakeVector (.X (Math|Vector|BreakVector _tetrisposition)) (.y _returnvalue_4) (.z _returnvalue_4))))))
      (Transformation|SetActorLocation (Math|Vector|Lerp(Vector) (Transformation|GetActorLocation) _output_get_2 _returnvalue_3) false false))
    (:then_1
      (Transformation|SetActorScale3D (Math|Vector|MakeVector (/ (Variables|/Script/Engine.SceneCaptureComponent2D|GetOrthoWidth (Variables|Default|GetSceneCaptureComponent2D)) (Variables|Default|GetTetrisOrtoSize)) (/ (Variables|/Script/Engine.SceneCaptureComponent2D|GetOrthoWidth (Variables|Default|GetSceneCaptureComponent2D)) (Variables|Default|GetTetrisOrtoSize)) (/ (Variables|/Script/Engine.SceneCaptureComponent2D|GetOrthoWidth (Variables|Default|GetSceneCaptureComponent2D)) (Variables|Default|GetTetrisOrtoSize)))))))

(fn ConstructionScript)