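; Combat controller actor that spawns the player, enemies and coins on tiles and registers itself with MainGameMode on BeginPlay.
; Spawn functions place actors at a small offset from the tile, storing enemies and coins in maps keyed by tile position.
; Enemy stats (base plus random-unit-vector-weighted increments), EXP reward and coin value scale exponentially with BlocksCreated from MainGameState, using StatGrowPerBlock.
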(event EventBeginPlay
  (Variables|/Game/Blueprints/MainGameMode.MainGameMode_C|SetCombat%20Controller (.AsMain%20Game%20Mode (Utilities|Casting|CastToMainGameMode (Game|GetGameMode))) self))

(event Collision|EventActorBeginOverlap
  (params (OtherActor :type Actor%20Object%20Reference)))

(event EventTick
  (params (DeltaSeconds :type Float%20%28single-precision%29)))

(fn ConstructionScript)

(fn SpawnEnemy
  (params (Tile :type Field%20Tile%20Object%20Reference))
  (bind _returnvalue (Transformation|GetActorTransform Tile))
  (bind _returnvalue_2 (Math|Random|RandomUnitVector))
  (bind _returnvalue_3 (Game|GetGameState))
  (bind _baseenemystats (Variables|Default|GetBaseEnemyStats))
  (bind _baseenemystats_randomincrement (Variables|Default|GetBaseEnemyStats_RandomIncrement))
  (bind _statgrowperblock (Variables|Default|GetStatGrowPerBlock))
  (bind _returnvalue_4 (Math|Vector|VectorGetAbs _returnvalue_2))
  (bind _asmain_game_state (Utilities|Casting|CastToMainGameState _returnvalue_3))
  (bind _blockscreated (Variables|/Game/Blueprints/MainGameState.MainGameState_C|GetBlocksCreated _asmain_game_state))
  (bind _returnvalue_5 (Math|Conversions|ToFloat(Integer) _blockscreated))
  (bind _returnvalue_6 (Math|Float|Power _statgrowperblock _returnvalue_5))
  (bind _returnvalue_7 (Game|SpawnActorfromClass "/Game/Blueprints/Combat/Enemy.Enemy_C" (Math|Transform|MakeTransform (+ (.location _returnvalue) "-25.000000, 0, 0") (.rotation _returnvalue) (.scale _returnvalue)) "Undefined" 0 0))
  (Variables|/Game/Blueprints/Combat/Combatant.Combatant_C|SetCombatStats _returnvalue_7 (Utilities|Struct|MakeCharStats (Math|Float|Truncate (* (+ (Math|Conversions|ToFloat(Integer) (.hp (.basestats _baseenemystats))) (* (Math|Conversions|ToFloat(Integer) (.hp _baseenemystats_randomincrement)) (.x _returnvalue_4))) _returnvalue_6)) (Math|Float|Truncate (* (+ (Math|Conversions|ToFloat(Integer) (.atk (.basestats _baseenemystats))) (* (Math|Conversions|ToFloat(Integer) (.atk _baseenemystats_randomincrement)) (.y _returnvalue_4))) _returnvalue_6)) (Math|Float|Truncate (* (+ (Math|Conversions|ToFloat(Integer) (.defence (.basestats _baseenemystats))) (* (Math|Conversions|ToFloat(Integer) (.defence _baseenemystats_randomincrement)) (.z _returnvalue_4))) _returnvalue_6))))
  (Variables|/Game/Blueprints/Combat/Enemy.Enemy_C|SetExp%20Reward _returnvalue_7 (* (.expreward _baseenemystats) _returnvalue_6))
  (Utilities|Map|Add (Variables|Default|GetEnemies) (Variables|/Game/Blueprints/FieldTile.FieldTile_C|GetPosition Tile) _returnvalue_7)
  (return _returnvalue_7))

(fn SpawnPlayer
  (params (Tile :type Field%20Tile%20Object%20Reference))
  (bind _returnvalue (Transformation|GetActorTransform Tile))
  (bind _returnvalue_2 (Game|SpawnActorfromClass "/Game/Blueprints/Combat/Player.Player_C" (Math|Transform|MakeTransform (+ (.location _returnvalue) "-25.000000, 0, 0") (.rotation _returnvalue) (.scale _returnvalue)) "Undefined" 0 0))
  (Variables|/Game/Blueprints/Combat/Player.Player_C|SetCurrentCell _returnvalue_2 Tile))

(fn SpawnCoin
  (params (Tile :type Field%20Tile%20Object%20Reference))
  (bind _returnvalue (Transformation|GetActorTransform Tile))
  (bind _returnvalue_2 (Game|SpawnActorfromClass "/Game/Blueprints/Combat/Coin.Coin_C" (Math|Transform|MakeTransform (+ (.location _returnvalue) "-25.000000, 0, 0") (.rotation _returnvalue) (.scale _returnvalue)) "Undefined" 0 0))
  (Variables|/Game/Blueprints/Combat/Coin.Coin_C|SetCost _returnvalue_2 (Math|Float|Truncate (* (Math|Float|Power (Variables|Default|GetStatGrowPerBlock) (Math|Conversions|ToFloat(Integer) (Variables|/Game/Blueprints/MainGameState.MainGameState_C|GetBlocksCreated (.AsMain%20Game%20State (Utilities|Casting|CastToMainGameState (Game|GetGameState)))))) 1e+01)))
  (Utilities|Map|Add (Variables|Default|GetCoins) (Variables|/Game/Blueprints/FieldTile.FieldTile_C|GetPosition Tile) _returnvalue_2))