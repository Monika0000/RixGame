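; Combatant Blueprint that runs automatic combat against another combatant using a CombatStats struct of HP, Atk and Defence.
; Attack loops AttackTick with a short Delay while either side is alive, so it only ends once both reach zero HP or below.
; Each tick damages both sides by the opponent's Atk minus own Defence, clamped at zero.
; Afterwards it calls OnDefeat, an empty function here, on each dead combatant.
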(event Custom|Attack
  (params (Other :type Combatant%20Object%20Reference))
  (while (or (CallFunction|IsAlive) (CallFunction|IsAlive Other))
    (CallFunction|AttackTick Other)
    (Utilities|FlowControl|Delay 0.3))
  (Utilities|FlowControl|Sequence
    (:then_0
      (if (not (CallFunction|IsAlive))
        (CallFunction|OnDefeat)))
    (:then_1
      (if (not (CallFunction|IsAlive Other))
        (CallFunction|OnDefeat Other)))))

(event EventBeginPlay)

(event Collision|EventActorBeginOverlap
  (params (OtherActor :type Actor%20Object%20Reference)))

(event EventTick
  (params (DeltaSeconds :type Float%20%28single-precision%29)))

(fn ConstructionScript)

(fn AttackTick
  (params (Other :type Combatant%20Object%20Reference))
  (Variables|Default|SetCombatStats (Utilities|Struct|MakeCharStats (- (.hp (Variables|Default|GetCombatStats)) (Math|Integer|Max(Integer) (- (.atk (Variables|Combatant_C|GetCombatStats Other)) (.defence (Variables|Default|GetCombatStats))))) (.atk (Variables|Default|GetCombatStats)) (.defence (Variables|Default|GetCombatStats))))
  (Variables|Combatant_C|SetCombatStats Other (Utilities|Struct|MakeCharStats (- (.hp (Variables|Combatant_C|GetCombatStats Other)) (Math|Integer|Max(Integer) (- (.atk (Variables|Default|GetCombatStats)) (.defence (Variables|Combatant_C|GetCombatStats Other))))) (.atk (Variables|Combatant_C|GetCombatStats Other)) (.defence (Variables|Combatant_C|GetCombatStats Other)))))

(fn OnDefeat)

(fn IsAlive
  (return (> (.hp (Variables|Default|GetCombatStats)) 0)))