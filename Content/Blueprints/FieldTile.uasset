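; FieldTile is a grid cell actor with a type (empty, monster, chest, random, wall, entry point) and two Paper2D sprites.
; SetTileType picks the main sprite for the type and flags walls as shut.
; SetTilePosition places the tile on the Y-Z plane, offset from its TileHolder by the game mode's cell size.
; Tick forces the wall sprite on shut tiles and shows one sprite or the other according to the game state's Tetris mode.
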(event EventBeginPlay)

(event Collision|EventActorBeginOverlap
  (params (OtherActor :type Actor%20Object%20Reference)))

(event EventTick
  (params (DeltaSeconds :type Float%20%28single-precision%29))
  (bind _returnvalue (Game|GetGameState))
  (bind _papersprite1 (Variables|Default|GetPaperSprite1))
  (bind _asmain_game_state (Utilities|Casting|CastToMainGameState _returnvalue))
  (bind _istetrismode (Variables|/Game/Blueprints/MainGameState.MainGameState_C|GetIsTetrisMode _asmain_game_state))
  (Utilities|FlowControl|Sequence
    (:then_0
      (if (Variables|Default|GetIsShut)
        (Rendering|Components|Sprite|SetSprite (Variables|Default|GetPaperSprite) "/Game/Sprites/TileUITetris/UI1_Sprite.UI1_Sprite")
        (Rendering|Components|Sprite|SetSprite _papersprite1 "/Game/Sprites/TileUITetris/UI1_Sprite.UI1_Sprite")))
    (:then_1
      (Rendering|SetVisibility (Variables|Default|GetPaperSprite) _istetrismode false)
      (Rendering|SetVisibility _papersprite1 (not _istetrismode) false))))

(fn ConstructionScript)

(fn SetTileType
  (params (Type :type TileType%20Enum :default "NewEnumerator0"))
  (bind _papersprite (Variables|Default|GetPaperSprite))
  (bind _output_get (Variables|Default|SetTileType Type))
  (switch Utilities|FlowControl|Switch|SwitchonTileType _output_get
    (:NewEnumerator0
      (Rendering|Components|Sprite|SetSprite _papersprite 0))
    (:NewEnumerator1
      (Rendering|Components|Sprite|SetSprite _papersprite "/Game/Sprites/TileUITetris/UI4_Sprite.UI4_Sprite"))
    (:NewEnumerator2
      (Rendering|Components|Sprite|SetSprite _papersprite "/Game/Sprites/TileUITetris/UI3_Sprite.UI3_Sprite"))
    (:NewEnumerator3
      (Rendering|Components|Sprite|SetSprite _papersprite "/Game/Sprites/TileUITetris/UI3_Sprite.UI3_Sprite"))
    (:NewEnumerator4
      (Rendering|Components|Sprite|SetSprite _papersprite "/Game/Sprites/TileUITetris/UI1_Sprite.UI1_Sprite")
      (Variables|Default|SetIsShut true))
    (:NewEnumerator6
      (Rendering|Components|Sprite|SetSprite _papersprite "/Game/Sprites/TileUITetris/UI0_Sprite.UI0_Sprite"))))

(fn SetTilePosition
  (params (Position :type Int%20Vector%202D%20Structure))
  (bind (_x _y) (Utilities|Struct|BreakIntVector2D Position))
  (bind _tileholder (Variables|Default|GetTileHolder))
  (bind _rootcomponent (Variables|/Script/Engine.Actor|GetRootComponent _tileholder))
  (bind _returnvalue (Transformation|GetWorldLocation _rootcomponent))
  (bind (_x_2 _y_2 _z) (Math|Vector|BreakVector _returnvalue))
  (Utilities|FlowControl|Sequence
    (:then_0
      (bind _asmain_game_mode (Utilities|Casting|CastToMainGameMode (Game|GetGameMode))
        (:CastFailed
          (Development|PrintString "Failed to cast MainGameMode!"))))
    (:then_1
      (if (Utilities|IsValid _tileholder)
        (Transformation|SetActorLocation (Math|Vector|MakeVector _x_2 (+ (Math|Conversions|ToFloat(Integer) (* (Variables|/Game/Blueprints/MainGameMode.MainGameMode_C|GetCellSize _asmain_game_mode) _x)) _y_2) (+ _z (Math|Conversions|ToFloat(Integer) (* _y (Variables|/Game/Blueprints/MainGameMode.MainGameMode_C|GetCellSize _asmain_game_mode))))) false false)
        (else
          (Development|PrintString "Tile holder is invalid!"))))
    (:then_2
      (Variables|Default|SetPosition Position))))