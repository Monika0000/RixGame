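; HUD_Testing is a debug actor that binds keyboard shortcuts to change MainGameState values for testing.
; Tab toggles the Tetris mode flag, number keys grant RixCoins or experience through AddExp, and plus and minus keys adjust the player's HP stat.
; Each handler casts the game state and edits it directly, rebuilding the PlayerStats struct with Atk and Defence preserved.
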(event EventBeginPlay)

(event Collision|EventActorBeginOverlap
  (params (OtherActor :type Actor%20Object%20Reference)))

(event EventTick
  (params (DeltaSeconds :type Float%20%28single-precision%29)))

(event Input|KeyboardEvents|1
  (params (Key :type Key%20Structure :default "None"))
  (bind _returnvalue (Game|GetGameState))
  (bind _asmain_game_state (Utilities|Casting|CastToMainGameState _returnvalue))
  (:Pressed
    (Variables|/Game/Blueprints/MainGameState.MainGameState_C|SetRixCoins _asmain_game_state (+ (Variables|/Game/Blueprints/MainGameState.MainGameState_C|GetRixCoins _asmain_game_state) 10))))

(event Input|KeyboardEvents|Subtract
  (params (Key :type Key%20Structure :default "None"))
  (:Pressed
    (bind _asmain_game_state (Utilities|Casting|CastToMainGameState (Game|GetGameState)))
    (Variables|/Game/Blueprints/MainGameState.MainGameState_C|SetPlayerStats _asmain_game_state (Utilities|Struct|MakeCharStats (+ (.hp (Variables|/Game/Blueprints/MainGameState.MainGameState_C|GetPlayerStats _asmain_game_state)) -1) (.atk (Variables|/Game/Blueprints/MainGameState.MainGameState_C|GetPlayerStats _asmain_game_state)) (.defence (Variables|/Game/Blueprints/MainGameState.MainGameState_C|GetPlayerStats _asmain_game_state))))))

(event Input|KeyboardEvents|Tab
  (params (Key :type Key%20Structure :default "None"))
  (bind _returnvalue (Game|GetGameState))
  (bind _asmain_game_state (Utilities|Casting|CastToMainGameState _returnvalue))
  (:Pressed
    (Variables|/Game/Blueprints/MainGameState.MainGameState_C|SetIsTetrisMode _asmain_game_state (not (Variables|/Game/Blueprints/MainGameState.MainGameState_C|GetIsTetrisMode _asmain_game_state)))))

(event Input|KeyboardEvents|2
  (params (Key :type Key%20Structure :default "None"))
  (:Pressed
    (bind _asmain_game_state (Utilities|Casting|CastToMainGameState (Game|GetGameState)))
    (Default|AddExp _asmain_game_state 1e+01)))

(event Input|KeyboardEvents|Add
  (params (Key :type Key%20Structure :default "None"))
  (:Pressed
    (bind _asmain_game_state (Utilities|Casting|CastToMainGameState (Game|GetGameState)))
    (Variables|/Game/Blueprints/MainGameState.MainGameState_C|SetPlayerStats _asmain_game_state (Utilities|Struct|MakeCharStats (+ (.hp (Variables|/Game/Blueprints/MainGameState.MainGameState_C|GetPlayerStats _asmain_game_state)) 1) (.atk (Variables|/Game/Blueprints/MainGameState.MainGameState_C|GetPlayerStats _asmain_game_state)) (.defence (Variables|/Game/Blueprints/MainGameState.MainGameState_C|GetPlayerStats _asmain_game_state))))))

(fn ConstructionScript)