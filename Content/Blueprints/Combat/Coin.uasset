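; Coin pickup with a Paper2D sprite that adds one to the RixCoins count when collected.
; Each tick it reads MainGameState and hides the sprite while Tetris mode is active.
; OnCollect increments the counter on MainGameState, and IsAlive reports whether CombatStats HP is above zero.
; The graphs shown contain no overlap handling or destroy logic.
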(event EventBeginPlay)

(event Collision|EventActorBeginOverlap
  (params (OtherActor :type Actor%20Object%20Reference)))

(event EventTick
  (params (DeltaSeconds :type Float%20%28single-precision%29))
  (Rendering|SetVisibility (Variables|Default|GetPaperSprite) (not (Variables|/Game/Blueprints/MainGameState.MainGameState_C|GetIsTetrisMode (.AsMain%20Game%20State (Utilities|Casting|CastToMainGameState (Game|GetGameState))))) false))

(fn ConstructionScript)

(fn OnCollect
  (bind _returnvalue (Game|GetGameState))
  (bind _asmain_game_state (Utilities|Casting|CastToMainGameState _returnvalue))
  (Variables|/Game/Blueprints/MainGameState.MainGameState_C|SetRixCoins _asmain_game_state (+ (Variables|/Game/Blueprints/MainGameState.MainGameState_C|GetRixCoins _asmain_game_state) 1)))

(fn IsAlive
  (return (> (.HP (Utilities|Struct|BreakCharStats (Variables|Default|GetCombatStats))) 0)))