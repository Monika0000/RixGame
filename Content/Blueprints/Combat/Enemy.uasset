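; Enemy actor for combat that shows its stats through a widget and grants experience when defeated.
; On BeginPlay it runs the parent logic, then sets itself as the Owner of the EnemyStatsDisplay in its Widget component.
; OnDefeat adds ExpReward to the MainGameState, marks OwnTile as shut, and destroys the actor after a short delay.
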(event EventBeginPlay
  (|CallParentFunction)
  (bind _asenemy_stats_display (Utilities|Casting|CastToEnemyStatsDisplay (UserInterface|GetUserWidgetObject (Variables|Default|GetWidget))))
  (Variables|/Game/Blueprints/Combat/EnemyStatsDisplay.EnemyStatsDisplay_C|SetOwner _asenemy_stats_display self))

(event Collision|EventActorBeginOverlap
  (params (OtherActor :type Actor%20Object%20Reference))
  (|CallParentFunction OtherActor) ; This node is disabled and will not be called.\nDrag off pins to build functionality.
)

(event EventTick
  (params (DeltaSeconds :type Float%20%28single-precision%29))
  (|CallParentFunction DeltaSeconds) ; This node is disabled and will not be called.\nDrag off pins to build functionality.
)

(event EventOnDefeat
  (bind _asmain_game_state (Utilities|Casting|CastToMainGameState (Game|GetGameState)))
  (Default|AddExp _asmain_game_state (Variables|Default|GetExp%20Reward))
  (Utilities|FlowControl|Sequence
    (:then_0
      (Utilities|FlowControl|Delay 0.1)
      (Actor|DestroyActor))
    (:then_1
      (Variables|/Game/Blueprints/FieldTile.FieldTile_C|SetIsShut (Variables|Default|GetOwnTile) true))))

(fn ConstructionScript
  (|CallParentFunction))