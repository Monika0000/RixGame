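; Game mode that serves as the factory for a grid-based playing field made of FieldShape and FieldTile actors.
; CreateTiles maps grid points to tiles spawned by CreateTile, which attaches each to its holder and swaps a placeholder type for a random one.
; CreateShape spawns and positions a shape, optionally retyping one random tile as the entry point.
; GetOffset returns the neighboring grid coordinate in a given direction.
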(event EventBeginPlay)

(event EventTick
  (params (DeltaSeconds :type Float%20%28single-precision%29)))

(fn ConstructionScript)

(fn GetOffset
  (params (Direction :type MoveDirection%20Enum :default "NewEnumerator0") (Position :type Int%20Vector%202D%20Structure))
  (bind (_x _y) (Utilities|Struct|BreakIntVector2D Position))
  (bind (_x_2 _y_2) (Utilities|Struct|BreakIntVector2D Position))
  (bind (_x_3 _y_3) (Utilities|Struct|BreakIntVector2D Position))
  (bind (_x_4 _y_4) (Utilities|Struct|BreakIntVector2D Position))
  (switch Utilities|FlowControl|Switch|SwitchonMoveDirection Direction
    (:NewEnumerator0
      (return (Utilities|Struct|MakeIntVector2D _x_2 (+ _y_2 1))))
    (:NewEnumerator1
      (return (Utilities|Struct|MakeIntVector2D _x_3 (+ _y_3 -1))))
    (:NewEnumerator2
      (return (Utilities|Struct|MakeIntVector2D (+ _x_4 -1) _y_4)))
    (:NewEnumerator3
      (return (Utilities|Struct|MakeIntVector2D (+ _x 1) _y)))))

(fn ChooseRandomTile
  (switch int (Math|Random|RandomIntegerinRange 1 3)
    (:Default
      (Development|PrintString "FieldShape::ChooseRandomTile() : incorrect number!"))
    (:0
      (return "NewEnumerator0"))
    (:1
      (return "NewEnumerator1"))
    (:2
      (return "NewEnumerator2"))
    (:3
      (return "NewEnumerator3"))))

(fn CreateTile
  (params (Holder :type Actor%20Object%20Reference) (TileType :type TileType%20Enum :default "NewEnumerator5") (Position :type Int%20Vector%202D%20Structure))
  (bind _returnvalue (Game|SpawnActorfromClass "/Game/Blueprints/FieldTile.FieldTile_C" (Math|Transform|MakeTransform "0, 0, 0") "Undefined" 0 0))
  (if (Utilities|Enum|Equal(Enum) TileType "NewEnumerator5")
    (bind _type (CallFunction|ChooseRandomTile))
    (Default|SetTileType _returnvalue _type)
    (else
      (Default|SetTileType _returnvalue TileType)))
  (Variables|/Game/Blueprints/FieldTile.FieldTile_C|SetTileHolder _returnvalue Holder)
  (Transformation|AttachActorToActor _returnvalue Holder "None" "KeepRelative" "KeepRelative" "KeepRelative" true)
  (Default|SetTilePosition _returnvalue Position)
  (return _returnvalue))

(fn CreateTiles
  (params (Holder :type Actor%20Object%20Reference) (TileType :type TileType%20Enum :default "NewEnumerator5") (Points :type Array%20of%20Int%20Vector%202D%20Structures))
  (Utilities|FlowControl|Sequence
    (:then_0
      (for _array_element Points
        (bind _tile (CallFunction|CreateTile Holder TileType _array_element))
        (Utilities|Map|Add (LocalVariables|GetOutTiles) _array_element _tile)))
    (:then_1
      (return (LocalVariables|GetOutTiles)))))

(fn CreateShape
  (params (Position :type Int%20Vector%202D%20Structure) (EntryPoint :type Boolean))
  (bind _returnvalue (Game|SpawnActorfromClass "/Game/Blueprints/FieldShape.FieldShape_C" (|InitPos) "Undefined" 0 0))
  (Default|SetPosition _returnvalue Position)
  (if EntryPoint
    (bind _keys (Utilities|Map|Keys (Variables|/Game/Blueprints/FieldShape.FieldShape_C|GetPoints _returnvalue)))
    (Default|SetTileType (.Value (Utilities|Map|Find (Variables|/Game/Blueprints/FieldShape.FieldShape_C|GetPoints _returnvalue) (Utilities|Array|Get(acopy) _keys (Math|Random|RandomIntegerinRange 0 (- (Utilities|Map|Length (Variables|/Game/Blueprints/FieldShape.FieldShape_C|GetPoints _returnvalue)) 1))))) "NewEnumerator6"))
  (return _returnvalue))