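; Tetris playfield actor that drops shapes on a timer while the game state is in Tetris mode and handles move and rotate keys.
; It builds a U-shaped wall into TileMap, the grid lookup used for collision checks.
; A shape blocked below hands its tiles to the field and is destroyed, and the next tick spawns another.
; Placed tiles of one type make the CombatController spawn an enemy.
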(event EventBeginPlay
  (Game|GetGameMode)
  (Variables|Default|SetFallTimePeriod (Variables|/Game/Blueprints/MainGameMode.MainGameMode_C|GetUpdatePeriod (Variables|Default|GetMainGameMode)))
  (CallFunction|InitWallTiles)
  (Variables|/Game/Blueprints/MainGameMode.MainGameMode_C|SetField (.AsMain%20Game%20Mode (Utilities|Casting|CastToMainGameMode (Game|GetGameMode))) self))

(event Collision|EventActorBeginOverlap
  (params (OtherActor :type Actor%20Object%20Reference)))

(event EventTick
  (params (DeltaSeconds :type Float%20%28single-precision%29))
  (if (Variables|/Game/Blueprints/MainGameState.MainGameState_C|GetIsTetrisMode (.AsMain%20Game%20State (Utilities|Casting|CastToMainGameState (Game|GetGameState))))
    (|DeltaTimeCycle DeltaSeconds (Variables|/Game/Blueprints/MainGameMode.MainGameMode_C|GetUpdatePeriod (Variables|Default|GetMainGameMode)))
    (CallFunction|CheckCollision)
    (if (Utilities|IsValid (Variables|Default|GetCurrentShape))
      (CallFunction|Move (Variables|Default|GetCurrentShape) "NewEnumerator1")
      (CallFunction|CheckCollision)
      (else
        (bind _shape (Default|CreateShape (Variables|Default|GetMainGameMode) (Utilities|Struct|MakeIntVector2D 0 5)))
        (Variables|Default|SetCurrentShape _shape)
        (CallFunction|CheckCollision)))))

(event Input|KeyboardEvents|D
  (params (Key :type Key%20Structure :default "None"))
  (bind _currentshape (Variables|Default|GetCurrentShape))
  (:Pressed
    (bind _result (CallFunction|IsCollide _currentshape "NewEnumerator3"))
    (if (not _result)
      (CallFunction|Move _currentshape "NewEnumerator3")
      (CallFunction|CheckCollision))))

(event Input|KeyboardEvents|S
  (params (Key :type Key%20Structure :default "None"))
  (bind _currentshape (Variables|Default|GetCurrentShape))
  (:Pressed
    (bind _result (CallFunction|IsCollide _currentshape "NewEnumerator1"))
    (if (not _result)
      (CallFunction|Move _currentshape "NewEnumerator1")
      (CallFunction|CheckCollision))))

(event Input|KeyboardEvents|A
  (params (Key :type Key%20Structure :default "None"))
  (bind _currentshape (Variables|Default|GetCurrentShape))
  (:Pressed
    (bind _result (CallFunction|IsCollide _currentshape "NewEnumerator2"))
    (if (not _result)
      (CallFunction|Move _currentshape "NewEnumerator2")
      (CallFunction|CheckCollision))))

(event Input|KeyboardEvents|R
  (params (Key :type Key%20Structure :default "None"))
  (bind _currentshape (Variables|Default|GetCurrentShape))
  (:Pressed
    (if (Utilities|IsValid _currentshape)
      (Utilities|FlowControl|Sequence
        (:then_0
          (Default|RotateShape _currentshape false))
        (:then_1
          (bind _result (CallFunction|IsCollide _currentshape "NewEnumerator1"))
          (if _result
            (Default|RotateShape _currentshape true)))
        (:then_2
          (CallFunction|CheckCollision))))))

(fn ConstructionScript)

(fn Move
  (params (Shape :type Field%20Shape%20Object%20Reference) (Direction :type MoveDirection%20Enum :default "NewEnumerator0"))
  (bind _position (Variables|/Game/Blueprints/FieldShape.FieldShape_C|GetPosition Shape))
  (bind _position_2 (Variables|/Game/Blueprints/FieldShape.FieldShape_C|GetPosition Shape))
  (bind _position_3 (Variables|/Game/Blueprints/FieldShape.FieldShape_C|GetPosition Shape))
  (bind _position_4 (Variables|/Game/Blueprints/FieldShape.FieldShape_C|GetPosition Shape))
  (bind (_x _y) (Utilities|Struct|BreakIntVector2D _position))
  (bind (_x_2 _y_2) (Utilities|Struct|BreakIntVector2D _position_2))
  (bind (_x_3 _y_3) (Utilities|Struct|BreakIntVector2D _position_3))
  (bind (_x_4 _y_4) (Utilities|Struct|BreakIntVector2D _position_4))
  (if (Utilities|IsValid Shape)
    (switch Utilities|FlowControl|Switch|SwitchonMoveDirection Direction
      (:NewEnumerator0
        (Default|SetPosition Shape (Utilities|Struct|MakeIntVector2D _x_2 (+ _y_2 1))))
      (:NewEnumerator1
        (Default|SetPosition Shape (Utilities|Struct|MakeIntVector2D _x_3 (+ _y_3 -1))))
      (:NewEnumerator2
        (Default|SetPosition Shape (Utilities|Struct|MakeIntVector2D (+ _x_4 -1) _y_4)))
      (:NewEnumerator3
        (Default|SetPosition Shape (Utilities|Struct|MakeIntVector2D (+ _x 1) _y))))))

(fn IsCollide
  (params (Shape :type Field%20Shape%20Object%20Reference) (Direction :type MoveDirection%20Enum :default "NewEnumerator0"))
  (bind _position (Variables|/Game/Blueprints/FieldShape.FieldShape_C|GetPosition Shape))
  (bind (_x _y) (Utilities|Struct|BreakIntVector2D _position))
  (if (Utilities|IsValid Shape)
    (bind _keys (Utilities|Map|Keys (Variables|/Game/Blueprints/FieldShape.FieldShape_C|GetPoints Shape)))
    (for _array_element _keys
      (bind _result (Default|GetOffset (Variables|Default|GetMainGameMode) Direction (Utilities|Struct|MakeIntVector2D (+ (.X (Utilities|Struct|BreakIntVector2D _array_element)) _x) (+ (.Y (Utilities|Struct|BreakIntVector2D _array_element)) _y))))
      (if (.ReturnValue (Utilities|Map|Find (Variables|Default|GetTileMap) _result))
        (return true))))
  (return false))

(fn InitWallTiles
  (Utilities|FlowControl|Sequence
    (:then_0
      (for _index (range -5 4)
        (Utilities|Array|Add (LocalVariables|GetWallPoints) (Utilities|Struct|MakeIntVector2D -3 _index))))
    (:then_1
      (for _index_2 (range -5 4)
        (Utilities|Array|Add (LocalVariables|GetWallPoints) (Utilities|Struct|MakeIntVector2D 4 _index_2))))
    (:then_2
      (for _index_3 (range -3 4)
        (Utilities|Array|Add (LocalVariables|GetWallPoints) (Utilities|Struct|MakeIntVector2D _index_3 -6))))
    (:then_3
      (bind _tiles (Default|CreateTiles (Variables|Default|GetMainGameMode) self "NewEnumerator4" (LocalVariables|GetWallPoints)))
      (Variables|Default|SetTileMap _tiles))))

(fn PlaceShape
  (params (Shape :type Field%20Shape%20Object%20Reference))
  (bind _position (Variables|/Game/Blueprints/FieldShape.FieldShape_C|GetPosition Shape))
  (bind (_x _y) (Utilities|Struct|BreakIntVector2D _position))
  (Utilities|FlowControl|Sequence
    (:then_0
      (bind _keys (Utilities|Map|Keys (Variables|/Game/Blueprints/FieldShape.FieldShape_C|GetPoints Shape)))
      (for _array_element _keys
        (Utilities|Map|Add (Variables|Default|GetTileMap) (Utilities|Struct|MakeIntVector2D (+ (.X (Utilities|Struct|BreakIntVector2D (Variables|/Game/Blueprints/FieldTile.FieldTile_C|GetPosition (.Value (Utilities|Map|Find (Variables|/Game/Blueprints/FieldShape.FieldShape_C|GetPoints Shape) _array_element))))) _x) (+ (.Y (Utilities|Struct|BreakIntVector2D (Variables|/Game/Blueprints/FieldTile.FieldTile_C|GetPosition (.Value (Utilities|Map|Find (Variables|/Game/Blueprints/FieldShape.FieldShape_C|GetPoints Shape) _array_element))))) _y)) (.Value (Utilities|Map|Find (Variables|/Game/Blueprints/FieldShape.FieldShape_C|GetPoints Shape) _array_element)))
        (Variables|/Game/Blueprints/FieldTile.FieldTile_C|SetTileHolder (.Value (Utilities|Map|Find (Variables|/Game/Blueprints/FieldShape.FieldShape_C|GetPoints Shape) _array_element)) self)
        (Transformation|AttachActorToActor (.Value (Utilities|Map|Find (Variables|/Game/Blueprints/FieldShape.FieldShape_C|GetPoints Shape) _array_element)) self "None" "KeepRelative" "KeepRelative" "KeepRelative" true)
        (Default|SetTilePosition (.Value (Utilities|Map|Find (Variables|/Game/Blueprints/FieldShape.FieldShape_C|GetPoints Shape) _array_element)) (Utilities|Struct|MakeIntVector2D (+ (.X (Utilities|Struct|BreakIntVector2D (Variables|/Game/Blueprints/FieldTile.FieldTile_C|GetPosition (.Value (Utilities|Map|Find (Variables|/Game/Blueprints/FieldShape.FieldShape_C|GetPoints Shape) _array_element))))) _x) (+ (.Y (Utilities|Struct|BreakIntVector2D (Variables|/Game/Blueprints/FieldTile.FieldTile_C|GetPosition (.Value (Utilities|Map|Find (Variables|/Game/Blueprints/FieldShape.FieldShape_C|GetPoints Shape) _array_element))))) _y)))
        (if (Utilities|Enum|Equal(Enum) (Variables|/Game/Blueprints/FieldTile.FieldTile_C|GetTileType (.Value (Utilities|Map|Find (Variables|/Game/Blueprints/FieldShape.FieldShape_C|GetPoints Shape) _array_element))) "NewEnumerator1")
          (Default|SpawnEnemy (Variables|/Game/Blueprints/MainGameMode.MainGameMode_C|GetCombat%20Controller (.AsMain%20Game%20Mode (Utilities|Casting|CastToMainGameMode (Game|GetGameMode)))) (.Value (Utilities|Map|Find (Variables|/Game/Blueprints/FieldShape.FieldShape_C|GetPoints Shape) _array_element))))))
    (:then_1
      (Actor|DestroyActor Shape))))

(fn CheckCollision
  (bind _result (CallFunction|IsCollide (Variables|Default|GetCurrentShape) "NewEnumerator1"))
  (if _result
    (CallFunction|PlaceShape (Variables|Default|GetCurrentShape))
    (Variables|Default|SetFallTimePeriod (Variables|/Game/Blueprints/MainGameMode.MainGameMode_C|GetUpdatePeriod (Variables|Default|GetMainGameMode)))))

(fn GetTile
  (params (Position :type Int%20Vector%202D%20Structure))
  (bind _tilemap (Variables|Default|GetTileMap))
  (bind (_value _returnvalue) (Utilities|Map|Find _tilemap Position))
  (return _value _returnvalue))