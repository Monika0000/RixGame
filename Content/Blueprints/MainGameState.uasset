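; MainGameState tracks the player's stats, experience and level, plus a count of blocks created as shapes are born.
; Adding experience checks a recursive Fibonacci-style threshold and triggers at most one level-up, which subtracts the cost and raises HP, attack and defence.
; Tick polls player HP and calls GameOver on MainGameMode once it is zero or below.
; The shape-placed handler is empty.
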(event Custom|OnShapeBorn
  (params (Shape :type Field%20Shape%20Object%20Reference))
  (Math|Integer|IncrementInt (Variables|Default|GetBlocksCreated)))

(event Custom|OnShapePlaced
  (params (Shape :type Field%20Shape%20Object%20Reference)))

(event EventBeginPlay)

(event EventTick
  (params (DeltaSeconds :type Float%20%28single-precision%29))
  (if (<= (.hp (Variables|Default|GetPlayerStats)) 0)
    (bind _asmain_game_mode (Utilities|Casting|CastToMainGameMode (Game|GetGameMode)))
    (Default|GameOver _asmain_game_mode)))

(fn ConstructionScript)

(fn CalculateLevelExp
  (params (Level :type Integer))
  (if (<= Level 0)
    (return 5.0)
    (else
      (return (+ (CallFunction|CalculateLevelExp (- Level 1)) (CallFunction|CalculateLevelExp (- Level 2)))))))

(fn PlayerLvlUP
  (bind _playerlevel (Variables|Default|GetPlayerLevel))
  (Variables|Default|SetExp (- (Variables|Default|GetExp) (CallFunction|CalculateLevelExp (Variables|Default|GetPlayerLevel))))
  (Math|Integer|IncrementInt _playerlevel
    (:%20%20
      (Variables|Default|SetPlayerStats (Utilities|Struct|MakeCharStats (+ (.hp (Variables|Default|GetPlayerStats)) _playerlevel) (+ (.atk (Variables|Default|GetPlayerStats)) 1) (+ (.defence (Variables|Default|GetPlayerStats)) 1))))))

(fn AddExp
  (params (Exp :type Float%20%28single-precision%29))
  (bind _output_get (Variables|Default|SetExp (+ Exp (Variables|Default|GetExp))))
  (if (>= _output_get (CallFunction|CalculateCurrentLevelExp))
    (CallFunction|PlayerLvlUP)))

(fn CalculateCurrentLevelExp
  (return (CallFunction|CalculateLevelExp (Variables|Default|GetPlayerLevel))))